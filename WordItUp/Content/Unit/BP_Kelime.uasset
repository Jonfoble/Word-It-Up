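; BP_Kelime is a word display actor that shows a randomly chosen word on its Kelime text element.
; On BeginPlay it waits briefly, caches the player controller, game instance and game mode, then picks a word; the ChangeKelime event re-rolls it.
; The game instance's Manuel flag selects the source: a random key from its KelimeDB map, or the Word field of a random data table row.
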(event `ChangeKelime`
  (if (`/Game/General/BP_GameInstance.Manuel` (`self.As BP Game Instance`)) :!label _label
    (bind _keys (`BlueprintMapLibrary.Map_Keys` (`/Game/General/BP_GameInstance.KelimeDB` (`self.As BP Game Instance`))))
    (bind _output_get (set `self.MyWord` (`KismetArrayLibrary.Array_Random` _keys)))
    (`TextRenderComponent.K2_SetText` (`self.Kelime`) (`KismetTextLibrary.Conv_StringToText` _output_get))
    (else
      ;[1 1 1] Hazır
      (bind _outrownames (`DataTableFunctionLibrary.GetDataTableRowNames` "/Game/Data/DATATable.DATATable"))
      (bind _returnvalue (`|GetDataTableRow` "/Game/Data/DATATable.DATATable" (`KismetArrayLibrary.Array_Random` _outrownames))
        (:`then`
          (`TextRenderComponent.K2_SetText` (`self.Kelime`) (`KismetTextLibrary.Conv_StringToText` (break `/Game/Data/S_DAta` _returnvalue))))))))

(event `self.ReceiveBeginPlay`
  (`KismetSystemLibrary.Delay` 0.2)
  (bind _asbp_player_controller_base (cast `/Game/General/BP_PlayerControllerBase` (`GameplayStatics.GetPlayerController` 0)))
  (set `self.As BP Player Controller Base` _asbp_player_controller_base)
  (bind _asbp_game_instance (cast `/Game/General/BP_GameInstance` (`GameplayStatics.GetGameInstance`)))
  (set `self.As BP Game Instance` _asbp_game_instance)
  (bind _asbp_game_mode_base (cast `/Game/General/BP_GameModeBase` (`GameplayStatics.GetGameMode`)))
  (set `self.As BP Game Mode Base` _asbp_game_mode_base)
  (goto _label))

(fn `UserConstructionScript`)