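; Base player controller that initializes health and score and spawns the game's UI widgets: menu, manual, scoreboard, pause, win and lose screens.
; The pause, win and lose screens pause the game.
; They and the manual set a shared WidgetOpened flag on BP_GameInstance, which is cached at BeginPlay.
; The Pause input opens the pause screen only while that flag is clear.
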(event `self.ReceiveBeginPlay`
  (set `self.Health` 100.0)
  (set `self.Skor` 0.0)
  (bind _asbp_game_instance (cast `/Game/General/BP_GameInstance` (`GameplayStatics.GetGameInstance`)))
  (set `self.As BP Game Instance` _asbp_game_instance))

(event `CreateScoreUI`
  (bind _returnvalue (`|CreateWidget` "/Game/UI/UI_SkorTablo.UI_SkorTablo_C"))
  (bind _output_get (set `self.Score_UI` _returnvalue))
  (`UserWidget.AddToViewport` _output_get 0))

(event `WinGame`
  (`GameplayStatics.SetGamePaused` true)
  (bind _returnvalue (`|CreateWidget` "/Game/UI/UI_Win.UI_Win_C"))
  (bind _output_get (set `self.WinUI` _returnvalue))
  (`UserWidget.AddToViewport` _output_get 0)
  (set `/Game/General/BP_GameInstance.WidgetOpened` true (`self.As BP Game Instance`)))

(event `InputAction|Pause`
  (params (Key :type "Key Structure"))
  (:`Pressed`
    (if (not (`/Game/General/BP_GameInstance.WidgetOpened` (`self.As BP Game Instance`)))
      (bind _returnvalue (`|CreateWidget` "/Game/UI/UI_Paused.UI_Paused_C"))
      (bind _output_get (set `self.Pause_UI` _returnvalue))
      (`UserWidget.AddToViewport` _output_get 0)
      (`GameplayStatics.SetGamePaused` true)
      (set `/Game/General/BP_GameInstance.WidgetOpened` true (`self.As BP Game Instance`)))))

(fn `CreateLoseUI`
  (bind _returnvalue (`|CreateWidget` "/Game/UI/UI_Lose.UI_Lose_C"))
  (`UserWidget.AddToViewport` _returnvalue 0)
  (set `/Game/General/BP_GameInstance.WidgetOpened` true (`self.As BP Game Instance`))
  (`GameplayStatics.SetGamePaused` true))

(fn `CreateManuelUI`
  (bind _returnvalue (`|CreateWidget` "/Game/UI/UI_Manuel.UI_Manuel_C"))
  (bind _output_get (set `self.Entry_UI` _returnvalue))
  (`UserWidget.AddToViewport` _output_get 0)
  (set `/Game/General/BP_GameInstance.WidgetOpened` true (`self.As BP Game Instance`)))

(fn `CreateMenuUI`
  (bind _returnvalue (`|CreateWidget` "/Game/UI/UI_Menu.UI_Menu_C"))
  (bind _output_get (set `self.Menu_UI` _returnvalue))
  (`UserWidget.AddToViewport` _output_get 0))

(fn `UserConstructionScript`)