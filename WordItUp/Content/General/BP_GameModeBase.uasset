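; Game mode for a balloon game that runs endless spawning of BoxBaloon actors and sets up mouse-driven play.
; On BeginPlay it switches to Game and UI input with a visible cursor, plays background music, and starts a self-repeating one-second delay loop.
; Each loop pass spawns a balloon at a randomly picked TargetPoint in the level, always spawning regardless of collision.
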(event `self.ReceiveBeginPlay`
  (bind _returnvalue (`GameplayStatics.GetPlayerController` 0))
  (`|ExecutionSequence`
    (:`then_0`
      (`WidgetBlueprintLibrary.SetInputMode_GameAndUIEx` _returnvalue null "DoNotLock" false)
      (set `PlayerController.bShowMouseCursor` true _returnvalue))
    (:`then_1`
      (`KismetSystemLibrary.Delay` 1.0)
      (`self.SpawnBaloon` :!label _label)
      (`KismetSystemLibrary.Delay` 1.0)
      (goto _label))
    (:`then_2`
      (`GameplayStatics.PlaySound2D` "/Game/Sound/BackgroundMusic.BackgroundMusic" 1.0 1.0 0.0 null null))))

(fn `GetRandomSpawnPoint`
  (returns (SpawnPoint :type "TargetPoint Object Reference"))
  (bind _outactors (`GameplayStatics.GetAllActorsOfClass` "/Script/Engine.TargetPoint"))
  (return (`KismetArrayLibrary.Array_Random` _outactors)))

(fn `SpawnBaloon`
  (bind _spawnpoint (`self.GetRandomSpawnPoint`))
  (`/Engine/EditorBlueprintResources/StandardMacros.IsValid` _spawnpoint
    (:`Is Valid`
      (`|SpawnActorFromClass` "/Game/Unit/BoxBaloon.BoxBaloon_C" (`self.GetTransform` _spawnpoint) "AlwaysSpawn" "OverrideRootScale" null "" 0.0 null))))

(fn `UserConstructionScript`)